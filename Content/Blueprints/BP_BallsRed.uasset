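; BP_BallsRed is a red ball actor that drifts from its spawn point toward the first-person character's starting location.
; Tick advances that lerp only while the character's BallsGoing flag is false.
; GoToWhite fires a one-shot timeline that pulls the ball toward the passed white ball.
; Overlapping a white ball prints a debug message, destroys both balls and clears the character's BallsGoing and ball-lock flags.
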(event `self.ReceiveBeginPlay`
  (`|ExecutionSequence`
    (:`then_0`
      (bind _outactors (`GameplayStatics.GetAllActorsOfClass` "/Game/Blueprints/BP_FirstPersonCharacter.BP_FirstPersonCharacter_C"))
      (bind _output_get (set `self.VRChar` (`KismetArrayLibrary.Array_Get` _outactors)))
      (set `self.VRCharPos` (`self.K2_GetActorLocation` _output_get)))
    (:`then_1`
      (bind _outactors_2 (`GameplayStatics.GetAllActorsOfClass` "/Game/Blueprints/BP_BallsWhite.BP_BallsWhite_C"))
      (set `self.whiteBall` (`KismetArrayLibrary.Array_Get` _outactors_2)))
    (:`then_2`
      (set `self.ballOrigin` (`SceneComponent.K2_GetComponentLocation` (`self.DefaultSceneRoot`))))))

(event `self.ReceiveTick`
  (params (DeltaSeconds :type "Float (single-precision)"))
  (if (not (`/Game/Blueprints/BP_FirstPersonCharacter.ballsGoing` (`self.VRChar`)))
    (set `self.ballPos` (`self.K2_GetActorLocation`))
    (bind _output_get (set `self.alpha` (+ (* (`GameplayStatics.GetWorldDeltaSeconds`) (`self.lerpSpeed`)) (`self.alpha`))))
    (`self.K2_SetActorLocation` (`KismetMathLibrary.VLerp` (`self.ballOrigin`) (`self.VRCharPos`) _output_get))))

(event `GoToWhite`
  (params (WhiteBall :type "/Game/Blueprints/BP_BallsWhite Object Reference"))
  (`/Engine/EditorBlueprintResources/StandardMacros.DoOnce` false
    (:`Completed`
      (bind (_direction _newtrack_4) (`Timeline|Timeline_0` :!via `PlayFromStart`)
        (:`Update`
          (`self.K2_SetActorLocation` (`KismetMathLibrary.VLerp` (`self.K2_GetActorLocation`) (`self.K2_GetActorLocation` WhiteBall) _newtrack_4)))))))

(event `self.Sphere.OnComponentBeginOverlap`
  (params (OtherActor :type "Actor Object Reference") (OtherComp :type "PrimitiveComponent Object Reference") (OtherBodyIndex :type Integer) (bFromSweep :type Boolean) (SweepResult :type "HitResult Structure (by ref)"))
  (bind _vrchar (`self.VRChar`))
  (bind _asbp_balls_white (cast `/Game/Blueprints/BP_BallsWhite` OtherActor))
  (`KismetSystemLibrary.PrintString` "RED EXPLODE")
  (`self.K2_DestroyActor`)
  (`self.K2_DestroyActor` _asbp_balls_white)
  (set `/Game/Blueprints/BP_FirstPersonCharacter.ballsGoing` false (`self.VRChar`))
  (set `/Game/Blueprints/BP_FirstPersonCharacter.redBallLocked` false _vrchar)
  (set `/Game/Blueprints/BP_FirstPersonCharacter.whiteBallLocked` false _vrchar))

(fn `UserConstructionScript`)