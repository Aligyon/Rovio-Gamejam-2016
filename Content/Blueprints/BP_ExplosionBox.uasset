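; BP_ExplosionBox is a box actor that explodes when its cube is hit by a first-person projectile.
; Explode fires a radial force impulse, activates two explosion components (detaching PExplosion so it stays in place), hides the cube, then destroys the actor after a short delay.
; Damage events do not trigger the explosion: AnyDamage only prints a debug string and RadialDamage is empty.
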(event `Explode`
  (bind _p_explosion (`self.P_Explosion`))
  (`RadialForceComponent.FireImpulse` (`self.RadialForce`))
  (`ActorComponent.Activate` _p_explosion false)
  (`SceneComponent.DetachFromParent` _p_explosion true true)
  (`SceneComponent.SetVisibility` (`self.Cube`) false false)
  (`ActorComponent.Activate` (`self.Explosion01`) false)
  (`KismetSystemLibrary.Delay` 3.0)
  (`self.K2_DestroyActor`))

(event `self.Cube.OnComponentHit`
  (params (OtherActor :type "Actor Object Reference") (OtherComp :type "PrimitiveComponent Object Reference") (NormalImpulse :type "Vector Structure") (Hit :type "HitResult Structure (by ref)"))
  (cast `/Game/Blueprints/BP_FirstPersonProjectile` OtherActor)
  (`self.Explode`))

(event `self.ReceiveRadialDamage`
  (params (DamageReceived :type "Float (single-precision)") (DamageType :type "DamageType Object Reference") (Origin :type "Vector Structure") (HitInfo :type "HitResult Structure (by ref)") (InstigatedBy :type "Controller Object Reference") (DamageCauser :type "Actor Object Reference")))

(event `self.ReceiveAnyDamage`
  (params (Damage :type "Float (single-precision)") (DamageType :type "DamageType Object Reference") (InstigatedBy :type "Controller Object Reference") (DamageCauser :type "Actor Object Reference"))
  (`KismetSystemLibrary.PrintString` "dmg"))

(fn `UserConstructionScript`)