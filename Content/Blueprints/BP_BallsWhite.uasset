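; White ball actor that flies toward the player character and can be sent into a red ball to explode.
; While the character's BallsGoing flag is off, Tick lerps it from its origin to the player's BeginPlay position, speeding up with game time.
; GoToRedBall runs a one-shot timeline toward the given red ball.
; Overlapping a red ball detonates, clears lock flags and destroys both; hitting the player zeroes HP.
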(event `self.ReceiveBeginPlay`
  ;[1 1 1] Start
  (`|ExecutionSequence`
    (:`then_0`
      (bind _outactors (`GameplayStatics.GetAllActorsOfClass` "/Game/Blueprints/BP_FirstPersonCharacter.BP_FirstPersonCharacter_C"))
      (bind _output_get (set `self.VRChar` (`KismetArrayLibrary.Array_Get` _outactors)))
      (set `self.VRCharPos` (`self.K2_GetActorLocation` _output_get)))
    (:`then_1`
      (bind _outactors_2 (`GameplayStatics.GetAllActorsOfClass` "/Game/Blueprints/BP_BallsRed.BP_BallsRed_C"))
      (set `self.ballRed` (`KismetArrayLibrary.Array_Get` _outactors_2)))
    (:`then_2`
      (set `self.ballOrigin` (`SceneComponent.K2_GetComponentLocation` (`self.DefaultSceneRoot`))))))

(event `self.ReceiveTick`
  (params (DeltaSeconds :type "Float (single-precision)"))
  ;[1 1 1] Going to Player
  (set `self.lerpSpeed` (* (`/Game/Blueprints/BP_FirstPersonCharacter.gameTime` (`self.VRChar`)) (`self.ballSpeedOverTime`)))
  (`|ExecutionSequence`
    (:`then_0`
      (if (not (`/Game/Blueprints/BP_FirstPersonCharacter.ballsGoing` (`self.VRChar`)))
        (set `self.ballPos` (`self.K2_GetActorLocation`))
        (bind _output_get (set `self.alpha` (+ (* (`GameplayStatics.GetWorldDeltaSeconds`) (`self.lerpSpeed`)) (`self.alpha`))))
        (`self.K2_SetActorLocation` (`KismetMathLibrary.VLerp` (`self.ballOrigin`) (`self.VRCharPos`) _output_get))))))

(event `GoToRedBall`
  (params (redBall :type "/Game/Blueprints/BP_BallsRed Object Reference"))
  ;[1 1 1] Going to Red Ball
  (`/Engine/EditorBlueprintResources/StandardMacros.DoOnce` false
    (:`Completed`
      (bind (_direction _newtrack_4) (`Timeline|Timeline_0` :!via `PlayFromStart`)
        (:`Update`
          (`self.K2_SetActorLocation` (`KismetMathLibrary.VLerp` (`self.K2_GetActorLocation`) (`self.K2_GetActorLocation` redBall) _newtrack_4)))))))

(event `self.Sphere.OnComponentBeginOverlap`
  (params (OtherActor :type "Actor Object Reference") (OtherComp :type "PrimitiveComponent Object Reference") (OtherBodyIndex :type Integer) (bFromSweep :type Boolean) (SweepResult :type "HitResult Structure (by ref)"))
  (bind _vrchar (`self.VRChar`))
  (bind _explosion_p_white_and_red (`self.Explosion_P_white_and_red`))
  ;[1 1 1] Collision, Destroy
  (`|ExecutionSequence`
    (:`then_0`
      (bind _asbp_balls_red (cast `/Game/Blueprints/BP_BallsRed` OtherActor))
      (`/Engine/EditorBlueprintResources/StandardMacros.DoOnce` false
        (:`Completed`
          (`ActorComponent.Activate` _explosion_p_white_and_red false)
          (`SceneComponent.DetachFromParent` _explosion_p_white_and_red true true)
          (`SceneComponent.SetVisibility` (`/Game/Blueprints/BP_BallsRed.ball` _asbp_balls_red) false false)
          (`SceneComponent.SetVisibility` (`self.ball`) false false)
          (`SceneComponent.SetVisibility` (`self.Sphere`) false false)
          (`SceneComponent.SetVisibility` (`/Game/Blueprints/BP_BallsRed.Sphere` _asbp_balls_red) false false)
          (set `/Game/Blueprints/BP_FirstPersonCharacter.ballsGoing` false _vrchar)
          (set `/Game/Blueprints/BP_FirstPersonCharacter.redBallLocked` false _vrchar)
          (set `/Game/Blueprints/BP_FirstPersonCharacter.whiteBallLocked` false _vrchar)
          (`KismetSystemLibrary.Delay` 1.0)
          (`self.K2_DestroyActor`)
          (`self.K2_DestroyActor` _asbp_balls_red))))
    (:`then_1`
      (bind _asbp_first_person_character (cast `/Game/Blueprints/BP_FirstPersonCharacter` OtherActor))
      (`/Engine/EditorBlueprintResources/StandardMacros.DecrementInt` (`/Game/Blueprints/BP_FirstPersonCharacter.HP` _asbp_first_person_character)
        (:`  `
          (set `/Game/Blueprints/BP_FirstPersonCharacter.HP` 0 _asbp_first_person_character)
          (`self.K2_DestroyActor`))))))

(fn `UserConstructionScript`)